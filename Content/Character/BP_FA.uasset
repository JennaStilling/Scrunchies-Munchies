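; BP_FA is the player character in a top-down eat-to-grow game, moved along fixed world axes through Enhanced Input.
; Size doubles as health: damage subtracts from it, and hitting a smaller BPI_Enemy eats it, adding the returned value.
; SizeCheck steps through progression thresholds to trigger UpgradeSize, but nothing in this graph calls it.
; Death and growth upgrades are print-string placeholders, and GetPlayerTransform exposes the actor's transform.
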(event `self.ReceiveBeginPlay`
  (bind _asplayer_controller (cast `PlayerController` (`self.GetController`)))
  (`EnhancedInputSubsystemInterface.AddMappingContext` (pcsubsystem `EnhancedInputLocalPlayerSubsystem` _asplayer_controller) "/Game/Character/Input/IMC_TopDown.IMC_TopDown" 0 (struct)))

(event `EnhancedInput|/Game/Character/Input/IA_Move`
  (params (ActionValue :type "Vector2D Structure") (ElapsedSeconds :type "Float (double-precision)") (TriggeredSeconds :type "Float (double-precision)") (InputAction :type "InputAction Object Reference" :default "/Game/Character/Input/IA_Move.IA_Move"))
  (:`Triggered`
    (`self.AddMovementInput` (1.0 0.0 0.0) ActionValue_X)
    (`self.AddMovementInput` (0.0 -1.0 0.0) ActionValue_Y)))

(event `/Game/Character/BPI_Player.Damage`
  (params (damage :type Integer))
  (bind _output_get (set `self.Size` (- (`self.Size`) damage)))
  (if (<= _output_get 0)
    (`self.Dies`)))

(event `self.ReceiveHit`
  (params (MyComp :type "PrimitiveComponent Object Reference") (Other :type "Actor Object Reference") (OtherComp :type "PrimitiveComponent Object Reference") (bSelfMoved :type Boolean) (HitLocation :type "Vector Structure") (HitNormal :type "Vector Structure") (NormalImpulse :type "Vector Structure") (Hit :type "HitResult Structure (by ref)"))
  (bind _asbpi_enemy (cast `/Game/Character/BPI_Enemy` Other))
  (bind _size (`/Game/Character/BPI_Enemy.getSize` _asbpi_enemy))
  (if (< _size (`self.Size`))
    (bind _feedamount (`/Game/Character/BPI_Enemy.eaten` _asbpi_enemy self))
    (set `self.Size` (+ _feedamount (`self.Size`)))))

(event `Dies`
  (`KismetSystemLibrary.PrintString` "Reset stuff, level or something ")
  (`KismetSystemLibrary.PrintString` "Probably asks a game manager to do that ")
  (`KismetSystemLibrary.PrintString` "or not i guess"))

(event `Size Check`
  (if (> (`self.Size`) (`|GetArrayItem` (`self.SizeProgressionMarks`) (`self.SizeProgression`)))
    (if (< (`self.SizeProgression`) (`KismetArrayLibrary.Array_Length` (`self.SizeProgressionMarks`)))
      (`self.Upgrade Size`)
      (`/Engine/EditorBlueprintResources/StandardMacros.IncrementInt` (`self.SizeProgression`)))))

(event `Upgrade Size`
  (`KismetSystemLibrary.PrintString` "boi grow")
  (`KismetSystemLibrary.PrintString` "probably zoom out a little"))

(fn `getPlayerTransform`
  (returns (transform :type "Transform Structure"))
  (return (`self.GetTransform`)))

(fn `UserConstructionScript`)