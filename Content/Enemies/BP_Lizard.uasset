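; BP_Lizard is a lizard enemy in a size-based eat-or-be-eaten food chain.
; Pawn sensing flags on the AI blackboard that it has seen the player (BP_FA) and whether it is at least as big.
; On capsule overlap it damages a player no bigger than itself, and destroys itself on touching a rat or snake.
; Eaten destroys it and returns its feed amount, while GetSize exposes its size.
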(event `self.PawnSensing.OnSeePawn`
  (params (Pawn :type "Pawn Object Reference"))
  (bind _returnvalue (`AIBlueprintHelperLibrary.GetBlackboard` (`AIBlueprintHelperLibrary.GetAIController` self)))
  (bind _asbp_fa (cast `/Game/Character/BP_FA` Pawn))
  (`BlackboardComponent.SetValueAsBool` _returnvalue "HasSeenPlayer" true)
  (`BlackboardComponent.SetValueAsBool` _returnvalue "IsBigger" (>= (`self.Size`) (`/Game/Character/BP_FA.Size` _asbp_fa))))

(event `self.Capsule.OnComponentBeginOverlap`
  (params (OverlappedComponent :type "PrimitiveComponent Object Reference") (OtherActor :type "Actor Object Reference") (OtherComp :type "PrimitiveComponent Object Reference") (OtherBodyIndex :type Integer) (bFromSweep :type Boolean) (SweepResult :type "HitResult Structure (by ref)"))
  (bind _asbp_fa (cast `/Game/Character/BP_FA` OtherActor)
    (:`then`
      (if (>= (`self.Size`) (`/Game/Character/BP_FA.Size` _asbp_fa))
        (`/Game/Character/BP_FA.Damage` _asbp_fa (`self.Damage`))))
    (:`CastFailed`
      (cast `/Game/Enemies/BP_Rat1` OtherActor
        (:`then`
          (`self.K2_DestroyActor`))
        (:`CastFailed`
          (cast `/Game/Enemies/BP_Snake` OtherActor)
          (`self.K2_DestroyActor`))))))

(fn `eaten`
  (params (eater :type "/Game/Character/BPI_Player Interface"))
  (returns (feedAmount :type Integer))
  (`self.K2_DestroyActor`)
  (return (`self.Feed Amount`)))

(fn `getSize`
  (returns (size :type Integer))
  (return (`self.Size`)))

(fn `UserConstructionScript`)